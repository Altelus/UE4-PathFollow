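; BP_SplineTest2 is a test Blueprint for editing and inspecting spline points through debug keys.
; F clears the spline and rebuilds it from the SplinePoints array, with each local position doubled.
; P prints world locations by point index, looping from 1 to the point count rather than from 0.
; An unconnected timeline holds path-following logic that would set a world location by distance along the spline, but it never runs.
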(event `Key|F`
  ;[1 1 1] Reset Points
  (:`Pressed`
    (`SplineComponent.ClearSplinePoints`)
    (for _array_element (`self.SplinePoints`)
      (`SplineComponent.AddSplineLocalPoint` (* _array_element 2.0)))))

(event `Key|P`
  ;[1 1 1] Print points
  (:`Pressed`
    (for _index (range 1 (+ (`SplineComponent.GetNumSplinePoints`) 1))
      (`KismetSystemLibrary.PrintString` (`KismetStringLibrary.Conv_VectorToString` (`SplineComponent.GetWorldLocationAtSplinePoint` _index))))))

(fn `UserConstructionScript`)
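; Key-driven test Blueprint for moving a static mesh along a spline and orienting it to the path.
; Z rebuilds the spline from a point array and draws it as debug points, as Q does.
; X replays a timeline to interpolate through a rotation array.
; C stops the plain follow timeline, then on release starts one that looks toward a point slightly ahead on the spline.
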(event `Key|X`
  (bind _returnvalue (+ (`self.i`) 1))
  (bind _returnvalue_2 (`KismetMathLibrary.Conv_VectorToRotator` (`KismetArrayLibrary.Array_Get` (`self.Rotations`) (`self.i`))))
  ;[1 1 1] Interpolate rotation at 0.5 sec intervals
  (:`Pressed`
    (set `self.i` 0)
    (bind (_direction _dt) (`Timeline|Timeline_1` :!label _label)
      (:`Update`
        (`SceneComponent.K2_SetWorldRotation` (`KismetMathLibrary.RInterpTo` (`self.prevRot`) _returnvalue_2 _dt 1.0)))
      (:`Finished`
        (if (< _returnvalue (`KismetArrayLibrary.Array_Length` (`self.Rotations`)))
          (set `self.prevRot` _returnvalue_2)
          (set `self.i` _returnvalue)
          (goto _label :!via `PlayFromStart`))))))

(event `Key|Q`
  (bind _di (`self.di`))
  ;[1 1 1] Draw spline1 debug points
  (:`Pressed`
    (set `self.di` 0.0 :!label _label_2)
    (while (<= _di (`SplineComponent.GetSplineLength`))
      (`KismetSystemLibrary.DrawDebugPoint` (`SplineComponent.GetWorldLocationAtDistanceAlongSpline` _di) 2.0 (struct :`G` 0.860821 :`B` 1.0 :`A` 1.0) 10.0)
      (set `self.di` (+ (`self.di`) 1.0)))
    (for _index (range (+ (`SplineComponent.GetNumSplinePoints`) 1))
      (`KismetSystemLibrary.DrawDebugPoint` (`SplineComponent.GetWorldLocationAtSplinePoint` _index) 5.0 (struct :`R` 1.0 :`B` 0.946138 :`A` 1.0) 10.0))))

(event `Key|C`
  ;[1 1 1] Interpolate rotation at 0.5 sec intervals
)

(event `self.ReceiveBeginPlay`)

(event `self.ReceiveActorBeginOverlap`
  (params (OtherActor :type "Actor Object Reference")))

(event `self.ReceiveTick`
  (params (DeltaSeconds :type "Float (single-precision)")))

(event `Key|Z`
  ;[1 1 1] Randomize and print points
  (:`Pressed`
    (if true
      (for _array_element _
        (`KismetSystemLibrary.PrintString` (`KismetStringLibrary.Conv_VectorToString` _array_element)))
      ;[1 1 1] Clear and load spline points from points array
      (`SplineComponent.ClearSplinePoints`)
      (for _array_element_2 _
        (`SplineComponent.AddSplineWorldPoint` _array_element_2))
      (goto _label_2))))

(event `Key|C`
  ;[1 1 1] Disable default path following, enable path following with look at
  (:`Pressed`
    ;[1 1 1] Move mesh along spline path
    (bind (_direction _dist) (`Timeline|Timeline_0` :!via `Stop`)
      (:`Update`
        (`SceneComponent.K2_SetWorldLocation` (`SplineComponent.GetWorldLocationAtDistanceAlongSpline` (* _dist (`SplineComponent.GetSplineLength` (`self.Spline1`))))))))
  (:`Released`
    (bind (_direction_2 _dist_2) (`Timeline|Timeline_2` :!via `PlayFromStart`)
      (:`Update`
        (bind _returnvalue (* _dist_2 (`SplineComponent.GetSplineLength` (`self.Spline1`))))
        (bind _returnvalue_2 (`SplineComponent.GetWorldLocationAtDistanceAlongSpline` (`self.Spline1`) _returnvalue))
        (`SceneComponent.K2_SetWorldLocation` (`self.StaticMesh1`) _returnvalue_2 false)
        (`SceneComponent.K2_SetWorldRotation` (`KismetMathLibrary.FindLookAtRotation` _returnvalue_2 (`SplineComponent.GetWorldLocationAtDistanceAlongSpline` (+ _returnvalue 10.0))))))))

(fn `UserConstructionScript`)